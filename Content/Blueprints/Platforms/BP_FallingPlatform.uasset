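; Falling platform actor that shakes and then shatters after the player steps into its overlap box.
; Five chained timelines lerp the actor's pitch back and forth before easing toward level.
; It then spawns and triggers an FS_MasterField at its location to break the geometry collection.
; After short delays it enables physics on the cube and collection, removes the cube, and finally destroys the actor.
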(event `self.Box.OnComponentBeginOverlap`
  (params (OverlappedComponent :type "PrimitiveComponent Object Reference") (OtherActor :type "Actor Object Reference") (OtherComp :type "PrimitiveComponent Object Reference") (OtherBodyIndex :type Integer) (bFromSweep :type Boolean) (SweepResult :type "HitResult Structure (by ref)"))
  ;[1 1 1] On begin overlap (Player to box)
  (if (== OtherActor (`GameplayStatics.GetPlayerCharacter` 0))
    (`self.RotatePlatform`)))

(event `SimulatePhysicsAndExplodePlatform`
  ;[1 1 1] Spawn master field delay simulate physics explode
  (bind _returnvalue (`|SpawnActorFromClass` "/Engine/EditorResources/FieldNodes/FS_MasterField.FS_MasterField_C" (`KismetMathLibrary.MakeTransform` (`self.K2_GetActorLocation`)) "Undefined" "MultiplyWithRoot" null null))
  (set `/Engine/EditorResources/FieldNodes/FS_MasterField.ActivationType` "NewEnumerator4" _returnvalue)
  (`/Engine/EditorResources/FieldNodes/FS_MasterField.CE_Trigger` _returnvalue)
  (`KismetSystemLibrary.Delay` 0.5)
  (`PrimitiveComponent.SetSimulatePhysics` (`self.Cube`) true)
  (`PrimitiveComponent.SetSimulatePhysics` (`self.GeometryCollection`) true)
  (`ActorComponent.K2_DestroyComponent` (`self.Cube`))
  (`KismetSystemLibrary.Delay` 5.0)
  (`self.K2_DestroyActor`))

(event `RotatePlatform`
  (bind (_returnvalue_roll _returnvalue_pitch _returnvalue_yaw) (`KismetMathLibrary.BreakRotator` (`self.K2_GetActorRotation`)))
  (bind (_returnvalue_roll_2 _returnvalue_pitch_2 _returnvalue_yaw_2) (`KismetMathLibrary.BreakRotator` (`self.K2_GetActorRotation`)))
  (bind (_returnvalue_roll_3 _returnvalue_pitch_3 _returnvalue_yaw_3) (`KismetMathLibrary.BreakRotator` (`self.K2_GetActorRotation`)))
  (bind (_returnvalue_roll_4 _returnvalue_pitch_4 _returnvalue_yaw_4) (`KismetMathLibrary.BreakRotator` (`self.K2_GetActorRotation`)))
  (bind (_returnvalue_roll_5 _returnvalue_pitch_5 _returnvalue_yaw_5) (`KismetMathLibrary.BreakRotator` (`self.K2_GetActorRotation`)))
  ;[1 1 1] Rotate platform from 10 to -10
  (bind (_direction _performshakingplatform) (`Timeline|Timeline` :!via `PlayFromStart`)
    (:`Update`
      (`self.K2_SetActorRotation` (`KismetMathLibrary.MakeRotator` _returnvalue_roll_2 (`KismetMathLibrary.Lerp` _returnvalue_pitch_2 10.0 _performshakingplatform) _returnvalue_yaw_2)))
    (:`Finished`
      (bind (_direction_2 _performshakingplatform_2) (`Timeline|Timeline_0` :!via `PlayFromStart`)
        (:`Update`
          (`self.K2_SetActorRotation` (`KismetMathLibrary.MakeRotator` _returnvalue_roll_3 (`KismetMathLibrary.Lerp` _returnvalue_pitch_3 -10.0 _performshakingplatform_2) _returnvalue_yaw_3)))
        (:`Finished`
          (bind (_direction_3 _performshakingplatform_3) (`Timeline|Timeline_1` :!via `PlayFromStart`)
            (:`Update`
              (`self.K2_SetActorRotation` (`KismetMathLibrary.MakeRotator` _returnvalue_roll_4 (`KismetMathLibrary.Lerp` _returnvalue_pitch_4 10.0 _performshakingplatform_3) _returnvalue_yaw_4)))
            (:`Finished`
              (bind (_direction_4 _performshakingplatform_4) (`Timeline|Timeline_2` :!via `PlayFromStart`)
                (:`Update`
                  (`self.K2_SetActorRotation` (`KismetMathLibrary.MakeRotator` _returnvalue_roll_5 (`KismetMathLibrary.Lerp` _returnvalue_pitch_5 -10.0 _performshakingplatform_4) _returnvalue_yaw_5)))
                (:`Finished`
                  (bind (_direction_5 _performshakingplatform_5) (`Timeline|Timeline_3` :!via `PlayFromStart`)
                    (:`Update`
                      (`self.K2_SetActorRotation` (`KismetMathLibrary.MakeRotator` _returnvalue_roll (`KismetMathLibrary.Lerp` _returnvalue_pitch 0.0 _performshakingplatform_5) _returnvalue_yaw)))
                    (:`Finished`
                      (`self.SimulatePhysicsAndExplodePlatform`))))))))))))

(fn `UserConstructionScript`)