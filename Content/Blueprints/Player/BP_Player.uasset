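; Player character with Enhanced Input movement, look and jump, an in-game pause menu and checkpoint respawning.
; On BeginPlay it adds the input mapping, stores its spawn transform and creates a hidden pause widget.
; The pause input toggles that widget, game pause, cursor and input mode.
; Respawn uses a timeline to scale the actor, teleport it to the last checkpoint, then reverse the scale; the explosion effects are unconnected.
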(event `self.ReceiveBeginPlay`
  ;[1 1 1] Call set mapping context - save transform - call create in game pause
  (`|ExecutionSequence`
    (:`then_0`
      (`self.SetMappingContext`))
    (:`then_1`
      (set `self.DefaultRespawnTransform` (`self.GetTransform`)))
    (:`then_2`
      (`self.CreateAndHidesInGamePauseWidget`))))

(event `CreateAndHidesInGamePauseWidget`
  ;[1 1 1] Create pause in game ref and hide it
  (bind _returnvalue (`|CreateWidget` "/Game/Blueprints/Widgets/WBP_InGamePause.WBP_InGamePause_C"))
  (bind _output_get (set `self.PauseMenuRef` _returnvalue))
  (set `/Game/Blueprints/Widgets/WBP_InGamePause.PlayerRef` self _output_get)
  (`UserWidget.AddToViewport` _output_get 0)
  (`Widget.SetVisibility` (`self.PauseMenuRef`) "Hidden")
  (set `self.IsPauseMenuDisplayed?` false))

(event `SetMappingContext`
  ;[1 1 1] Set mapping context
  (bind _asplayer_controller (cast `PlayerController` (`self.GetController`)))
  (bind _returnvalue (pcsubsystem `EnhancedInputLocalPlayerSubsystem` _asplayer_controller))
  (`/Engine/EditorBlueprintResources/StandardMacros.IsValid` _returnvalue
    (:`Is Valid`
      (`EnhancedInputSubsystemInterface.AddMappingContext` _returnvalue "/Game/Blueprints/Inputs/IMC_Player.IMC_Player" 0 (struct)))))

(event `ResumeFromInGamePause`
  (bind _returnvalue (`GameplayStatics.GetPlayerController` 0))
  ;[1 1 1] Pause in game
  (set `self.IsPauseMenuDisplayed?` false :!label _label)
  (`Widget.SetVisibility` (`self.PauseMenuRef`) "Hidden")
  (`WidgetBlueprintLibrary.SetInputMode_GameOnly` _returnvalue)
  (set `PlayerController.bShowMouseCursor` false _returnvalue)
  (`GameplayStatics.SetGamePaused` false))

(event `EnhancedInput|/Game/Blueprints/Inputs/Actions/IA_PauseInGame`
  (params (ActionValue :type Boolean) (ElapsedSeconds :type "Float (double-precision)") (TriggeredSeconds :type "Float (double-precision)") (InputAction :type "InputAction Object Reference" :default "/Game/Blueprints/Inputs/Actions/IA_PauseInGame.IA_PauseInGame"))
  (bind _returnvalue (`GameplayStatics.GetPlayerController` 0))
  (bind _pausemenuref (`self.PauseMenuRef`))
  ;[1 1 1] Pause in game
  (:`Started`
    (if (`self.IsPauseMenuDisplayed?`)
      (goto _label)
      (else
        (set `self.IsPauseMenuDisplayed?` true)
        (`Widget.SetVisibility` _pausemenuref "Visible")
        (`WidgetBlueprintLibrary.SetInputMode_GameAndUIEx` _returnvalue _pausemenuref)
        (set `PlayerController.bShowMouseCursor` true _returnvalue)
        (`GameplayStatics.SetGamePaused` true)))))

(event `EnhancedInput|/Game/Blueprints/Inputs/Actions/IA_MyLook`
  (params (ActionValue :type "Vector2D Structure") (ElapsedSeconds :type "Float (double-precision)") (TriggeredSeconds :type "Float (double-precision)") (InputAction :type "InputAction Object Reference" :default "/Game/Blueprints/Inputs/Actions/IA_MyLook.IA_MyLook"))
  ;[1 1 1] Move & Look input
  (:`Triggered`
    (`self.AddControllerYawInput` ActionValue_X)
    (`self.AddControllerPitchInput` ActionValue_Y)))

(event `EnhancedInput|/Game/Blueprints/Inputs/Actions/IA_MyJump`
  (params (ActionValue :type Boolean) (ElapsedSeconds :type "Float (double-precision)") (TriggeredSeconds :type "Float (double-precision)") (InputAction :type "InputAction Object Reference" :default "/Game/Blueprints/Inputs/Actions/IA_MyJump.IA_MyJump"))
  ;[1 1 1] Move & Look input
  (:`Started`
    (`self.Jump`))
  (:`Completed`
    (`self.StopJumping`)))

(event `EnhancedInput|/Game/Blueprints/Inputs/Actions/IA_MyMove`
  (params (ActionValue :type "Vector2D Structure") (ElapsedSeconds :type "Float (double-precision)") (TriggeredSeconds :type "Float (double-precision)") (InputAction :type "InputAction Object Reference" :default "/Game/Blueprints/Inputs/Actions/IA_MyMove.IA_MyMove"))
  (bind (_returnvalue_roll _returnvalue_pitch _returnvalue_yaw) (`KismetMathLibrary.BreakRotator` (`self.GetControlRotation`)))
  (bind (_returnvalue_roll_2 _returnvalue_pitch_2 _returnvalue_yaw_2) (`KismetMathLibrary.BreakRotator` (`self.GetControlRotation`)))
  ;[1 1 1] Move & Look input
  (:`Triggered`
    (`self.AddMovementInput` (`KismetMathLibrary.GetRightVector` (`KismetMathLibrary.MakeRotator` 0.0 0.0 _returnvalue_yaw_2)) ActionValue_X)
    (`self.AddMovementInput` (`KismetMathLibrary.GetForwardVector` (`KismetMathLibrary.MakeRotator` 0.0 0.0 _returnvalue_yaw)) ActionValue_Y)))

(event `SetNewCheckpointRespawnTransform`
  (params (NewTransformToSet :type "Transform Structure"))
  ;[1 1 1] Set new respawn transform / respawn VFX
  (set `self.DefaultRespawnTransform` NewTransformToSet))

(event `Respawn`
  (bind (_defaultrespawntransform_location _defaultrespawntransform_rotation) (`KismetMathLibrary.BreakTransform` (`self.DefaultRespawnTransform`)))
  ;[1 1 1] Set new respawn transform / respawn VFX
  (bind (_direction _scalevalue) (`Timeline|SetScaleTo0` :!via `PlayFromStart` :!label _label_2)
    (:`Update`
      (`self.SetActorScale3D` (`KismetMathLibrary.MakeVector` _scalevalue _scalevalue _scalevalue)))
    (:`Finished`
      (`self.K2_SetActorTransform` (`KismetMathLibrary.MakeTransform` _defaultrespawntransform_location _defaultrespawntransform_rotation (`self.GetActorScale3D`)) false true)
      (if (not (== (`self.GetActorScale3D`) (1.0 1.0 1.0) :`ErrorTolerance` 0.1))
        (goto _label_2 :!via `ReverseFromEnd`)))))

(fn `UserConstructionScript`)