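; BP_CylinderBumps is a bumper trap that launches the player on contact.
; When the player character overlaps its Capsule, a fixed world-space velocity-change impulse pushes the character diagonally upward, regardless of approach direction, and a 2D sound plays.
; The construction script gives the Cone and Sphere meshes randomly selected platform color materials.
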(event `self.Capsule.OnComponentBeginOverlap`
  (params (OverlappedComponent :type "PrimitiveComponent Object Reference") (OtherActor :type "Actor Object Reference") (OtherComp :type "PrimitiveComponent Object Reference") (OtherBodyIndex :type Integer) (bFromSweep :type Boolean) (SweepResult :type "HitResult Structure (by ref)"))
  (bind _returnvalue (`GameplayStatics.GetPlayerCharacter` 0))
  (if (== OtherActor _returnvalue)
    (`CharacterMovementComponent.AddImpulse` (`Character.CharacterMovement` _returnvalue) (1000.0 1000.0 1000.0) true)
    (`GameplayStatics.PlaySound2D` "/Engine/EditorSounds/Notifications/CompileFailed.CompileFailed" 1.0 1.0 0.0 null null)))

(fn `UserConstructionScript`
  (`PrimitiveComponent.SetMaterial` (`self.Cone`) 0 (select `int` (`KismetMathLibrary.RandomIntegerInRange` 0 5) :`0` "/Game/Blueprints/Materials/M_PlatformsColors_Blue.M_PlatformsColors_Blue" :`1` "/Game/Blueprints/Materials/M_PlatformsColors_Brown.M_PlatformsColors_Brown" :`2` "/Game/Blueprints/Materials/M_PlatformsColors_Green.M_PlatformsColors_Green" :`3` "/Game/Blueprints/Materials/M_PlatformsColors_Purple.M_PlatformsColors_Purple" :`4` "/Game/Blueprints/Materials/M_PlatformsColors_Red.M_PlatformsColors_Red" :`5` "/Game/Blueprints/Materials/M_PlatformsColors_Yellow.M_PlatformsColors_Yellow" :!type "MaterialInterface Object Reference"))
  (`PrimitiveComponent.SetMaterial` (`self.Sphere`) 0 (select `int` (`KismetMathLibrary.RandomIntegerInRange` 0 5) :`0` "/Game/Blueprints/Materials/M_PlatformsColors_Blue.M_PlatformsColors_Blue" :`1` "/Game/Blueprints/Materials/M_PlatformsColors_Brown.M_PlatformsColors_Brown" :`2` "/Game/Blueprints/Materials/M_PlatformsColors_Green.M_PlatformsColors_Green" :`3` "/Game/Blueprints/Materials/M_PlatformsColors_Purple.M_PlatformsColors_Purple" :`4` "/Game/Blueprints/Materials/M_PlatformsColors_Red.M_PlatformsColors_Red" :`5` "/Game/Blueprints/Materials/M_PlatformsColors_Yellow.M_PlatformsColors_Yellow" :!type "MaterialInterface Object Reference")))