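; BP_Tuto is a tutorial trigger that shows a message on screen while the player character is inside its sphere.
; On begin overlap it creates a WBP_Tuto widget, passes it the TutoText variable, stores the reference and adds it to the viewport.
; On end overlap it removes the stored widget and clears the reference.
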(event `self.Sphere.OnComponentBeginOverlap`
  (params (OverlappedComponent :type "PrimitiveComponent Object Reference") (OtherActor :type "Actor Object Reference") (OtherComp :type "PrimitiveComponent Object Reference") (OtherBodyIndex :type Integer) (bFromSweep :type Boolean) (SweepResult :type "HitResult Structure (by ref)"))
  (if (== OtherActor (`GameplayStatics.GetPlayerCharacter` 0))
    (bind _returnvalue (`|CreateWidget` "/Game/Blueprints/Widgets/WBP_Tuto.WBP_Tuto_C" null (`self.TutoText`)))
    (bind _output_get (set `self.TutoRef` _returnvalue))
    (`UserWidget.AddToViewport` _output_get 0)))

(event `self.Sphere.OnComponentEndOverlap`
  (params (OverlappedComponent :type "PrimitiveComponent Object Reference") (OtherActor :type "Actor Object Reference") (OtherComp :type "PrimitiveComponent Object Reference") (OtherBodyIndex :type Integer))
  (bind _tutoref (`self.TutoRef`))
  (if (== OtherActor (`GameplayStatics.GetPlayerCharacter` 0))
    (`/Engine/EditorBlueprintResources/StandardMacros.IsValid` _tutoref
      (:`Is Valid`
        (`Widget.RemoveFromParent` _tutoref)
        (set `self.TutoRef` null)))))

(fn `UserConstructionScript`)