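; BP_Coins is a collectible coin pickup that awards score to the player on touch.
; On BeginPlay it randomizes its starting yaw and spin rate through a RotatingMovement component.
; When CoinCol overlaps BP_Player, it calls AddScore, attaches a Niagara coin shower to the player's pelvis, plays a 2D sound and destroys itself.
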(event `self.ReceiveBeginPlay`
  (set `RotatingMovementComponent.RotationRate` (`KismetMathLibrary.MakeRotator` 0.0 0.0 (`KismetMathLibrary.RandomFloatInRange` 100.0 250.0)) (`self.RotatingMovement`))
  (`self.K2_SetActorRotation` (`KismetMathLibrary.MakeRotator` 0.0 0.0 (`KismetMathLibrary.RandomFloatInRange` 0.0 360.0))))

(event `self.CoinCol.OnComponentBeginOverlap`
  (params (OverlappedComponent :type "PrimitiveComponent Object Reference") (OtherActor :type "Actor Object Reference") (OtherComp :type "PrimitiveComponent Object Reference") (OtherBodyIndex :type Integer) (bFromSweep :type Boolean) (SweepResult :type "HitResult Structure (by ref)"))
  (bind _asbp_player (cast `/Game/Blueprints/Player/BP_Player` OtherActor))
  (`/Game/Blueprints/Player/BP_Player.AddScore` _asbp_player (`self.ScoreToAdd`))
  (`NiagaraFunctionLibrary.SpawnSystemAttached` "/Game/sA_PickupSet_1/Fx/NiagaraSystems/NS_Coin_Shower.NS_Coin_Shower" (`Character.Mesh` _asbp_player) "pelvis" (200.0 0.0 0.0) (struct :`Roll` 90.0) "KeepRelativeOffset")
  (`GameplayStatics.PlaySound2D` "/Engine/EditorSounds/Notifications/CompileSuccess.CompileSuccess" 1.0 1.0 0.0 null null)
  (`self.K2_DestroyActor`))

(fn `UserConstructionScript`)